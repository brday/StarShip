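; Interactive panel actor that shows a fixable state, turning green when repaired.
; Overlap begin and end set an InTrigger flag, toggle the text render's visibility and call the Buttontrue or Buttonfalse dispatcher to signal presence.
; The setFixed event swaps the panel to a green hex-tile material, plays a confirmation sound at world origin and prints a fixed message.
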(event Custom|setFixed
  (Rendering|Material|SetMaterial (Variables|Default|GetPanel) 0 "/Game/StarterContent/Materials/M_Tech_Hex_Tile_Green.M_Tech_Hex_Tile_Green")
  (Audio|PlaySoundatLocation "/Game/Sounds/ok.ok" "0, 0, 0")
  (Development|PrintString "Panel has been fixed."))

(event EventActorBeginOverlap
  (params (OtherActor :type Actor%20Object%20Reference))
  (Variables|Default|SetinTrigger true)
  (if (Variables|Default|GetinTrigger)
    (Rendering|ToggleVisibility (Variables|Default|GetTextRender1) false)
    (Default|CallButtontrue)
    (else
      (Rendering|ToggleVisibility (Variables|Default|GetTextRender1) false)
      (Default|CallButtonfalse))))

(event EventActorEndOverlap
  (params (OtherActor :type Actor%20Object%20Reference))
  (Variables|Default|SetinTrigger false)
  (if (Variables|Default|GetinTrigger)
    (Rendering|ToggleVisibility (Variables|Default|GetTextRender1) false)
    (Default|CallButtontrue)
    (else
      (Rendering|ToggleVisibility (Variables|Default|GetTextRender1) false)
      (Default|CallButtonfalse))))

(fn ConstructionScript)