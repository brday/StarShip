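; Turbolift actor that moves the player to another level, named by its DestinationLevel variable.
; Overlap events on its TriggerVolume enable input for player controller 0 on entry and disable it on exit, with no check on the overlapping actor.
; Pressing F plays the Turbolift sound at the actor's location, then opens the destination level after a fixed delay.
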(event OnComponentBeginOverlap(TriggerVolume)
  (params (OtherActor :type Actor%20Object%20Reference) (OtherComp :type Primitive%20Component%20Object%20Reference) (OtherBodyIndex :type Integer) (bFromSweep :type Boolean) (SweepResult :type Hit%20Result%20Structure%20%28by%20ref%29))
  (Input|EnableInput (Game|GetPlayerController 0)))

(event OnComponentEndOverlap(TriggerVolume)
  (params (OtherActor :type Actor%20Object%20Reference) (OtherComp :type Primitive%20Component%20Object%20Reference) (OtherBodyIndex :type Integer))
  (Input|DisableInput (Game|GetPlayerController 0)))

(event Input|KeyboardEvents|F
  (:Pressed
    (Audio|PlaySoundatLocation "/Game/Sounds/turbolift.turbolift" (Transformation|GetActorLocation))
    (Utilities|FlowControl|Delay 1e+01)
    (Game|OpenLevel(byName) (Utilities|String|StringToName (Variables|Default|GetDestinationLevel)))))

(fn ConstructionScript)