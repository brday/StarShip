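; Interactive warp trigger that lets the player press E to warp, ending in a transition to the Credits level.
; Overlapping the trigger volume enables input and leaving disables it, with both events toggling the text render's visibility.
; Releasing E plays the warp sound at world origin, prints a message and swaps the screen mesh to the warp material, then opens Credits after a delay.
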(event OnComponentBeginOverlap(TriggerVolume)
  (params (OtherActor :type Actor%20Object%20Reference) (OtherComp :type Primitive%20Component%20Object%20Reference) (OtherBodyIndex :type Integer) (bFromSweep :type Boolean) (SweepResult :type Hit%20Result%20Structure%20%28by%20ref%29))
  ;[1 1 1] Allow/Disallow Keyboard Input
  (Input|EnableInput (Game|GetPlayerController 0))
  (Rendering|ToggleVisibility (Variables|Default|GetTextRender1) false))

(event OnComponentEndOverlap(TriggerVolume)
  (params (OtherActor :type Actor%20Object%20Reference) (OtherComp :type Primitive%20Component%20Object%20Reference) (OtherBodyIndex :type Integer))
  ;[1 1 1] Allow/Disallow Keyboard Input
  (Input|DisableInput (Game|GetPlayerController 0))
  (Rendering|ToggleVisibility (Variables|Default|GetTextRender1) false))

(event Input|KeyboardEvents|E
  ;[1 1 1] Warp
  (:Released
    (Audio|PlaySoundatLocation "/Game/Sounds/warp.warp" "0, 0, 0")
    (Development|PrintString "Warping to nearest starbase!")
    (Rendering|Material|SetMaterial (Variables|/Script/Engine.StaticMeshActor|GetStaticMeshComponent (Variables|Default|GetScreen)) 0 "/Game/Textures/warp_Mat.warp_Mat")
    (Utilities|FlowControl|Delay 8.0)
    (Game|OpenLevel(byName) "Credits")))

(fn ConstructionScript)