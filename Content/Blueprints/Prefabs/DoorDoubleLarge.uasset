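; Large sliding double door prefab that opens automatically when something overlaps its trigger, unless Locked is set.
; Begin overlap plays a door sound and runs a timeline that lerps DoorL between start and end, with Door mirroring it by negation.
; End overlap reverses the timeline to close the doors, without sound.
; The construction script fills the number and name text from DoorNumber and DoorName.
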(event OnComponentBeginOverlap(DoorTrigger)
  (params (OtherActor :type Actor%20Object%20Reference) (OtherComp :type Primitive%20Component%20Object%20Reference) (OtherBodyIndex :type Integer) (bFromSweep :type Boolean) (SweepResult :type Hit%20Result%20Structure%20%28by%20ref%29))
  (if (not (Variables|Default|GetLocked))
    (Audio|PlaySoundatLocation "/Game/Sounds/doors.doors" (Transformation|GetActorLocation))
    (bind _openamount (Timeline|DoorOpenTimeline Play)
      (:Update
        (Transformation|SetRelativeLocation (Variables|Default|GetDoorL) (Math|Vector|Lerp(Vector) (Variables|Default|GetDoorStart) (Variables|Default|GetDoorEnd) _openamount) false)
        (Transformation|SetRelativeLocation (Variables|Default|GetDoor) (* (Math|Vector|Lerp(Vector) (Variables|Default|GetDoorStart) (Variables|Default|GetDoorEnd) _openamount) -1.0) false)))))

(event OnComponentEndOverlap(DoorTrigger)
  (params (OtherActor :type Actor%20Object%20Reference) (OtherComp :type Primitive%20Component%20Object%20Reference) (OtherBodyIndex :type Integer))
  (bind _openamount (Timeline|DoorOpenTimeline Reverse)
    (:Update
      (Transformation|SetRelativeLocation (Variables|Default|GetDoorL) (Math|Vector|Lerp(Vector) (Variables|Default|GetDoorStart) (Variables|Default|GetDoorEnd) _openamount) false)
      (Transformation|SetRelativeLocation (Variables|Default|GetDoor) (* (Math|Vector|Lerp(Vector) (Variables|Default|GetDoorStart) (Variables|Default|GetDoorEnd) _openamount) -1.0) false))))

(fn ConstructionScript
  (Rendering|Components|TextRender|SetText (Variables|Default|GetNumber) (Variables|Default|GetDoorNumber))
  (Rendering|Components|TextRender|SetText (Variables|Default|GetName) (Variables|Default|GetDoorName)))