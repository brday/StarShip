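; TurboLift is a turbolift prefab whose two doors swing open when something overlaps its trigger, unless it is locked.
; On begin overlap it plays a door sound and runs a timeline that rotates the left and right doors in opposite, mirrored directions.
; End overlap reverses the timeline to close the doors, with no lock check or sound.
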(event OnComponentBeginOverlap(Trigger)
  (params (OtherActor :type Actor%20Object%20Reference) (OtherComp :type Primitive%20Component%20Object%20Reference) (OtherBodyIndex :type Integer) (bFromSweep :type Boolean) (SweepResult :type Hit%20Result%20Structure%20%28by%20ref%29))
  (if (not (Variables|Default|GetLocked))
    (Audio|PlaySoundatLocation "/Game/Sounds/doors.doors" (Transformation|GetActorLocation))
    (bind _doorsopen (Timeline|TurboliftOpen Play)
      (:Update
        (Transformation|SetRelativeRotation (Variables|Default|GetdoorRight) (* (Math|Rotator|Lerp(Rotator) "0, 0, 0" "0.000000,34.000000, 0" _doorsopen) -1.0) false)
        (Transformation|SetRelativeRotation (Variables|Default|GetdoorLeft) (Math|Rotator|Lerp(Rotator) "0, 0, 0" "0.000000,34.000000, 0" _doorsopen) false)))))

(event OnComponentEndOverlap(Trigger)
  (params (OtherActor :type Actor%20Object%20Reference) (OtherComp :type Primitive%20Component%20Object%20Reference) (OtherBodyIndex :type Integer))
  (bind _doorsopen (Timeline|TurboliftOpen Reverse)
    (:Update
      (Transformation|SetRelativeRotation (Variables|Default|GetdoorRight) (* (Math|Rotator|Lerp(Rotator) "0, 0, 0" "0.000000,34.000000, 0" _doorsopen) -1.0) false)
      (Transformation|SetRelativeRotation (Variables|Default|GetdoorLeft) (Math|Rotator|Lerp(Rotator) "0, 0, 0" "0.000000,34.000000, 0" _doorsopen) false))))

(fn ConstructionScript)