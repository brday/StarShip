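; Interactive panel actor that reacts when any actor enters or leaves its overlap area.
; Begin and end overlap set the InTrigger flag and share one branch that flips TextRender1's visibility either way.
; The branch then fires CallButtontrue on entry or CallButtonfalse on exit.
; Visibility is toggled relative to its current state, and overlapping actors are neither filtered nor counted.
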(event EventActorBeginOverlap
  (params (OtherActor :type Actor%20Object%20Reference))
  ;[1 1 1] Comment
  (Variables|Default|SetinTrigger true)
  (if (Variables|Default|GetinTrigger)
    (Rendering|ToggleVisibility (Variables|Default|GetTextRender1) false)
    (Default|CallButtontrue)
    (else
      (Rendering|ToggleVisibility (Variables|Default|GetTextRender1) false)
      (Default|CallButtonfalse))))

(event EventActorEndOverlap
  (params (OtherActor :type Actor%20Object%20Reference))
  ;[1 1 1] Comment
  (Variables|Default|SetinTrigger false)
  (if (Variables|Default|GetinTrigger)
    (Rendering|ToggleVisibility (Variables|Default|GetTextRender1) false)
    (Default|CallButtontrue)
    (else
      (Rendering|ToggleVisibility (Variables|Default|GetTextRender1) false)
      (Default|CallButtonfalse))))

(fn ConstructionScript)